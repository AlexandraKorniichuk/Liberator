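; Parent Blueprint for food stand products that shows item name, price and weight text when the player is near.
; BeginPlay appends the item's values to the existing label text through AddStringToText.
; Actor overlaps with BP_ThirdPersonCharacter toggle ItemInfo visibility, propagated to its child components.
; PickUp is an empty event with no behavior in this Blueprint.
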(event `self.ReceiveBeginPlay`
  ;[0 0.1021 1] Init Above Texts
  (`self.Add String To Text` (`self.Item Info`) (`self.Item Name`))
  (`self.Add String To Text` (`self.PriceText`) (`KismetStringLibrary.Conv_DoubleToString` (`self.Item Price`)))
  (`self.Add String To Text` (`self.WeightText`) (`KismetStringLibrary.Conv_DoubleToString` (`self.Item Weight`))))

(event `self.ReceiveActorBeginOverlap`
  (params (OtherActor :type "Actor Object Reference"))
  (`self.Set Above Texts Visibility If Player` true OtherActor))

(event `self.ReceiveActorEndOverlap`
  (params (OtherActor :type "Actor Object Reference"))
  (`self.Set Above Texts Visibility If Player` false OtherActor))

(event `/Game/Products/FoodStand_Interface.Pick Up`)

(fn `Add String To Text`
  (params (`Text to change` :type "TextRenderComponent Object Reference") (String :type String))
  (`TextRenderComponent.K2_SetText` `Text to change` (`KismetTextLibrary.Conv_StringToText` (`KismetStringLibrary.Concat_StrStr` (`KismetTextLibrary.Conv_TextToString` (`TextRenderComponent.Text` `Text to change`)) String))))

(fn `Set Above Texts Visibility If Player`
  (params (NewVisibility :type Boolean) (OverlapActor :type "Actor Object Reference"))
  (cast `/Game/Blueprints/Player/Blueprints/BP_ThirdPersonCharacter` OverlapActor)
  (`SceneComponent.SetVisibility` (`self.Item Info`) NewVisibility true))

(fn `UserConstructionScript`)