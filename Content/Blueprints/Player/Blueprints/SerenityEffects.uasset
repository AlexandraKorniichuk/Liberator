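; Player component that provides audio feedback when the Serenity value is low.
; BeginPlay spawns a heartbeat sound, paused, at the owner's location and stores it.
; UpdateSerenityEffects takes a Serenity value and, below a hardcoded threshold, unpauses the heartbeat and adds a low-serenity effect to the music submix.
; At or above the threshold, it pauses the heartbeat and clears the submix effects.
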(event `self.ReceiveBeginPlay`
  (bind _returnvalue (`GameplayStatics.SpawnSoundAtLocation` "/Game/Sounds/SFX/Serenity/Heartbeat_SFX_Cue.Heartbeat_SFX_Cue" (`SceneComponent.K2_GetComponentLocation` (`Actor.RootComponent` (`self.GetOwner`))) (struct) 1.0 1.0 0.0 null null))
  (`AudioComponent.SetPaused` _returnvalue true)
  (set `self.Heartbeat_SFX` _returnvalue))

(fn `UpdateSerenityEffects`
  (params (Serenity :type "Float (double-precision)"))
  (bind _returnvalue (>= Serenity 90.0))
  (`AudioComponent.SetPaused` (`self.Heartbeat_SFX`) _returnvalue)
  (if _returnvalue
    (`AudioMixerBlueprintLibrary.ClearSubmixEffects` "/Game/Sounds/SFX/Serenity/MusicSubmix.MusicSubmix")
    (else
      (`AudioMixerBlueprintLibrary.AddSubmixEffect` "/Game/Sounds/SFX/Serenity/MusicSubmix.MusicSubmix" "/Game/Sounds/SFX/Serenity/LowSerenitySubmix.LowSerenitySubmix"))))