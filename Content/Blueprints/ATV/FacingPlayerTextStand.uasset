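; An actor that shows floating texts above itself while the third-person player character overlaps it, and hides them when the overlap ends.
; Begin and end overlap events share one function that ignores other actors and toggles the TextsAbove component and its children.
; The same call turns the texts toward the player by look-at yaw only, so facing updates on overlap changes rather than every tick.
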(event `self.ReceiveBeginPlay`
  (`parent.ReceiveBeginPlay`))

(event `self.ReceiveActorBeginOverlap`
  (params (OtherActor :type "Actor Object Reference"))
  (`self.Set Above Texts Visibility If Player` true OtherActor))

(event `self.ReceiveActorEndOverlap`
  (params (OtherActor :type "Actor Object Reference"))
  (`self.Set Above Texts Visibility If Player` false OtherActor))

(fn `Set Above Texts Visibility If Player`
  (params (NewVisibility :type Boolean) (OverlapActor :type "Actor Object Reference"))
  (bind _textsabove (`self.TextsAbove`))
  (bind (_returnvalue_roll _returnvalue_pitch _returnvalue_yaw) (`KismetMathLibrary.BreakRotator` (`KismetMathLibrary.FindLookAtRotation` (`SceneComponent.K2_GetComponentLocation` _textsabove) (`self.K2_GetActorLocation` (`self.Player`)))))
  (cast `/Game/Blueprints/Player/Blueprints/BP_ThirdPersonCharacter` OverlapActor)
  (`SceneComponent.SetVisibility` _textsabove NewVisibility true)
  (`SceneComponent.K2_SetWorldRotation` _textsabove (`KismetMathLibrary.MakeRotator` 0.0 0.0 _returnvalue_yaw) false false))

(fn `UserConstructionScript`
  (`parent.UserConstructionScript`))