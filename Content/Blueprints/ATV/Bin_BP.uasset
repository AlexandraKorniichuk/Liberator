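; Bin actor that shows a floating "Throw Out" prompt with a green "T" key hint when the player is nearby.
; BeginPlay fills both widget components through their AboveText widgets.
; Actor overlap begin and end toggle TextsAbove visibility, propagated to children, only for BP_ThirdPersonCharacter.
; The PickUp event is empty, so this graph holds no throw-out logic.
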(event `self.ReceiveBeginPlay`
  (bind _text (`self.GetAboveTextFromWiget` (`self.TextsAbove1`)))
  (`/Game/Blueprints/ATV/AboveText.SetColor` _text (make `SlateColor` (struct :`G` 0.766667 :`B` 0.02964 :`A` 1.0)))
  (`/Game/Blueprints/ATV/AboveText.SetText` _text (`KismetTextLibrary.Conv_StringToText` "T"))
  (`/Game/Blueprints/ATV/AboveText.SetText` (`self.GetAboveTextFromWiget` (`self.TextsAbove`)) (`KismetTextLibrary.Conv_StringToText` "Throw Out")))

(event `self.ReceiveActorBeginOverlap`
  (params (OtherActor :type "Actor Object Reference"))
  (`self.Set Above Texts Visibility If Player` true OtherActor))

(event `self.ReceiveActorEndOverlap`
  (params (OtherActor :type "Actor Object Reference"))
  (`self.Set Above Texts Visibility If Player` false OtherActor))

(event `/Game/Blueprints/ATV/Stand_Interface.Pick Up`)

(fn `GetAboveTextFromWiget`
  (params (NewParam :type "WidgetComponent Object Reference"))
  (returns (Text :type "/Game/Blueprints/ATV/AboveText Object Reference"))
  (bind _asabove_text (cast `/Game/Blueprints/ATV/AboveText` (`WidgetComponent.GetWidget` NewParam)))
  (return _asabove_text))

(fn `Set Above Texts Visibility If Player`
  (params (NewVisibility :type Boolean) (OverlapActor :type "Actor Object Reference"))
  (cast `/Game/Blueprints/Player/Blueprints/BP_ThirdPersonCharacter` OverlapActor)
  (`SceneComponent.SetVisibility` (`self.TextsAbove`) NewVisibility true))

(fn `UserConstructionScript`)