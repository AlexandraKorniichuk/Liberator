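; Parent Blueprint for food stand items with a name, price and weight, shown as text above the item.
; BeginPlay appends those values to the preset text labels and caches the player character.
; Player overlap shows or hides ItemInfo and its children, turning it in yaw toward the player only when an overlap begins or ends.
; PickUp is an empty event in this class.
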(event `self.ReceiveBeginPlay`
  ;[0 0.1021 1] Init Above Texts
  (`self.Add String To Text` (`self.Item Info`) (`self.Item Name`))
  (`self.Add String To Text` (`self.PriceText`) (`KismetStringLibrary.Conv_DoubleToString` (`self.Item Price`)))
  (`self.Add String To Text` (`self.WeightText`) (`KismetStringLibrary.Conv_DoubleToString` (`self.Item Weight`)))
  (bind _asbp_third_person_character (cast `/Game/Blueprints/Player/Blueprints/BP_ThirdPersonCharacter` (`GameplayStatics.GetPlayerCharacter` 0)))
  (set `self.Player` _asbp_third_person_character))

(event `self.ReceiveActorBeginOverlap`
  (params (OtherActor :type "Actor Object Reference"))
  (`self.Set Above Texts Visibility If Player` true OtherActor))

(event `self.ReceiveActorEndOverlap`
  (params (OtherActor :type "Actor Object Reference"))
  (`self.Set Above Texts Visibility If Player` false OtherActor))

(event `/Game/Blueprints/ATV/Stand_Interface.Pick Up`)

(fn `Add String To Text`
  (params (`Text to change` :type "TextRenderComponent Object Reference") (String :type String))
  (`TextRenderComponent.K2_SetText` `Text to change` (`KismetTextLibrary.Conv_StringToText` (`KismetStringLibrary.Concat_StrStr` (`KismetTextLibrary.Conv_TextToString` (`TextRenderComponent.Text` `Text to change`)) String))))

(fn `Set Above Texts Visibility If Player`
  (params (NewVisibility :type Boolean) (OverlapActor :type "Actor Object Reference"))
  (bind _item_info (`self.Item Info`))
  (bind (_returnvalue_roll _returnvalue_pitch _returnvalue_yaw) (`KismetMathLibrary.BreakRotator` (`KismetMathLibrary.RInterpTo` (`SceneComponent.K2_GetComponentRotation` (`self.Item Info`)) (`KismetMathLibrary.FindLookAtRotation` (`self.K2_GetActorLocation`) (`self.K2_GetActorLocation` (`self.Player`))) (`GameplayStatics.GetWorldDeltaSeconds`))))
  (cast `/Game/Blueprints/Player/Blueprints/BP_ThirdPersonCharacter` OverlapActor)
  (`SceneComponent.SetVisibility` _item_info NewVisibility true)
  (`SceneComponent.K2_SetWorldRotation` _item_info (`KismetMathLibrary.MakeRotator` 0.0 0.0 _returnvalue_yaw) false false))

(fn `UserConstructionScript`)