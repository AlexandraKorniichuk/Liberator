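; AI controller for a stationary watcher, apparently a security camera, that reports the player for stealing.
; Three perception components update a shared CanSeePlayer flag from sensing the player.
; Tick flags the theft on the player and plays a reaction sound when a suspicious player is seen, latched by SawStealing.
; InitAIPerception, not called here, selects one sight component for higher player Dexterity tiers.
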(event `self.ReceiveBeginPlay`
  (bind _asbp_third_person_character (cast `/Game/Blueprints/Player/Blueprints/BP_ThirdPersonCharacter` (`GameplayStatics.GetPlayerCharacter` 0)))
  (set `self.Player` _asbp_third_person_character))

(event `self.AIPerception_Dex1.OnTargetPerceptionUpdated`
  (params (Actor :type "Actor Object Reference") (Stimulus :type "AIStimulus Structure"))
  (cast `/Game/Blueprints/Player/Blueprints/BP_ThirdPersonCharacter` Actor)
  (set `self.CanSeePlayer` Stimulus_bSuccessfullySensed))

(event `self.AIPerception_Dex5.OnTargetPerceptionUpdated`
  (params (Actor :type "Actor Object Reference") (Stimulus :type "AIStimulus Structure"))
  (cast `/Game/Blueprints/Player/Blueprints/BP_ThirdPersonCharacter` Actor)
  (set `self.CanSeePlayer` Stimulus_bSuccessfullySensed))

(event `self.AIPerception_Dex10.OnTargetPerceptionUpdated`
  (params (Actor :type "Actor Object Reference") (Stimulus :type "AIStimulus Structure"))
  (cast `/Game/Blueprints/Player/Blueprints/BP_ThirdPersonCharacter` Actor)
  (set `self.CanSeePlayer` Stimulus_bSuccessfullySensed))

(event `self.ReceiveTick`
  (params (DeltaSeconds :type "Float (single-precision)"))
  (if (`self.SeeCrime`)
    (set `/Game/Blueprints/Player/Blueprints/BP_ThirdPersonCharacter.WasStealingReported` true (`self.Player`))
    (set `self.SawStealing` true)
    (`GameplayStatics.PlaySoundAtLocation` "/Game/Sounds/SFX/CameraStealingReaction.CameraStealingReaction" (0.0 0.0 0.0) (struct) 1.0 1.0 0.0 null null null null)))

(fn `InitAIPerception`
  (bind _dexterity (`/Game/Blueprints/Player/Blueprints/BP_ThirdPersonCharacter.Dexterity` (`self.Player`)))
  (if (== _dexterity 10)
    (`self.SetOneVisionEnabled` (`self.AIPerception_Dex10`))
    (elif (>= _dexterity 5)
      (`self.SetOneVisionEnabled` (`self.AIPerception_Dex5`)))))

(fn `SeeCrime`
  (returns (SeeCrime :type Boolean))
  (return (and (`self.CanSeePlayer`) (and (`/Game/Blueprints/Player/Blueprints/BP_ThirdPersonCharacter.IsSuspicious` (`self.Player`)) (not (`self.SawStealing`))))))

(fn `SetOneVisionEnabled`
  (params (EnabledPerception :type "AIPerceptionComponent Object Reference"))
  (for _array_element (`self.K2_GetComponentsByClass` "/Script/AIModule.AIPerceptionComponent")
    (`AIPerceptionComponent.SetSenseEnabled` _array_element "/Script/AIModule.AISense_Sight" (== null EnabledPerception))))

(fn `UserConstructionScript`)