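; Behavior tree task that copies the player's suspicion state into the AI's blackboard.
; On execute it casts player character 0 to BP_ThirdPersonCharacter and writes its IsSuspicious flag to the SawStealing key of the controlled pawn's blackboard.
; It prints a debug "Player is suspicious" message on every run, whatever the flag's value, then finishes with success.
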(event `self.ReceiveExecuteAI`
  (params (OwnerController :type "AIController Object Reference") (ControlledPawn :type "Pawn Object Reference"))
  (`self.InitPlayer`)
  (`KismetSystemLibrary.PrintString` "Player is suspicious")
  (`BlackboardComponent.SetValueAsBool` (`AIBlueprintHelperLibrary.GetBlackboard` ControlledPawn) "SawStealing" (`/Game/Blueprints/Player/Blueprints/BP_ThirdPersonCharacter.IsSuspicious` (`self.Player`)))
  (`self.FinishExecute` true))

(fn `InitPlayer`
  (bind _asbp_third_person_character (cast `/Game/Blueprints/Player/Blueprints/BP_ThirdPersonCharacter` (`GameplayStatics.GetPlayerCharacter` 0)))
  (set `self.Player` _asbp_third_person_character)
  (return))